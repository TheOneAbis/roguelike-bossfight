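; Wave manager that runs successive waves of patrol enemies, starting on BeginPlay and stopping after the maximum wave.
; Each wave spawns AI at random offsets within every spawn area, with the count scaling by the area's X/Y scale and the wave number.
; It binds to each spawned enemy's killed dispatcher and counts down, launching the next wave when the count reaches zero.
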(event `self.ReceiveBeginPlay`
  (`self.Begin First Wave`))

(event `OnEnemyKilled`
  (bind _currentwave (`self.currentWave`))
  (bind _result (`/Engine/EditorBlueprintResources/StandardMacros.DecrementInt` (`self.enemyCount`))
    (:`  `
      (if (<= _result 0)
        (bind _result_2 (`/Engine/EditorBlueprintResources/StandardMacros.IncrementInt` _currentwave :!label _label)
          (:`  `
            (if (not (> _currentwave (`self.maxWaves`)))
              (bind _spawned_enemies (`self.Spawn Enemies` _result_2))
              (for _array_element _spawned_enemies
                (add `/Game/Blueprints/BP_Damageable.OnKilledDispatch` _array_element (delegate `OnEnemyKilled`)))
              (set `self.enemyCount` (`KismetArrayLibrary.Array_Length` _spawned_enemies)))))))))

(event `Begin First Wave`
  (if (not (`self.started`))
    (set `self.started` true)
    (goto _label)))

(event `self.ReceiveTick`
  (params (DeltaSeconds :type "Float (single-precision)")))

(fn `Spawn Enemies`
  (params (Wave :type Integer))
  (returns (`Spawned Enemies` :type "Array of /Game/Blueprints/BP_Damageable Object Reference"))
  (locals (spawnedEnemies :type "Array of /Game/Blueprints/BP_Damageable Object Reference"))
  (for _array_element (`self.Spawn Areas`)
    (bind _rootcomponent (`Actor.RootComponent` _array_element))
    (bind (_returnvalue_x _returnvalue_y) (`KismetMathLibrary.BreakVector` (`SceneComponent.K2_GetComponentScale` _rootcomponent)))
    (for _ (range (+ (`KismetMathLibrary.FTrunc` (/ (* _returnvalue_x _returnvalue_y) (/ 1.0 (`KismetMathLibrary.Conv_IntToDouble` Wave) 2e-06))) 1))
      (bind _returnvalue (/ _returnvalue_x 2.0))
      (bind _returnvalue_2 (/ _returnvalue_y 2.0))
      (bind _returnvalue_3 (`AIBlueprintHelperLibrary.SpawnAIFromClass` "/Game/Blueprints/Enemies/BP_Enemy_Patrol.BP_Enemy_Patrol_C" null (+ (`SceneComponent.K2_GetComponentLocation` _rootcomponent) (`KismetMathLibrary.MakeVector` (`KismetMathLibrary.RandomFloatInRange` (* _returnvalue -1.0) _returnvalue) (`KismetMathLibrary.RandomFloatInRange` (* _returnvalue_2 -1.0) _returnvalue_2))) (struct) false self))
      (bind _asbp_damageable (cast `/Game/Blueprints/BP_Damageable` _returnvalue_3))
      (`KismetArrayLibrary.Array_Add` (`local.spawnedEnemies`) _asbp_damageable)))
  (return (`local.spawnedEnemies`)))

(fn `UserConstructionScript`)