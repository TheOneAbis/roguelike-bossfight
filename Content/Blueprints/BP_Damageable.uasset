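; BP_Damageable is a damageable actor Blueprint that tracks health, immunity and death, described in its comments as an enemy.
; The construction script sets CurrentHP to MaxHP, and TakeDamage subtracts from it unless Immune, setting Dead and calling the on-killed dispatcher at zero or below.
; A separate DeathMenu event shows the EndScene widget with a mouse cursor and pauses the game.
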(event `Set Immune`
  (params (Immune :type Boolean))
  (set `self.Immune` Immune))

(event `Take Damage`
  (params (damage :type "Float (double-precision)"))
  (bind _current_hp (`self.current HP`))
  ;[1 0.4531 0.4531] Taking damage. If hp <= 0, this enemy is dead and destroyed.
  (if (not (`self.Immune`))
    (set `self.current HP` (- _current_hp damage))
    (if (<= _current_hp 0.0)
      (set `self.Dead` true)
      (`self.OnKilledDispatch`)
      (else
        (set `self.Dead` false)))))

(event `DeathMenu`
  (bind _returnvalue (`|CreateWidget` "/Game/UI/EndScene.EndScene_C"))
  (bind _output_get (set `self.NewVar` _returnvalue))
  (`UserWidget.AddToViewport` _output_get 0)
  (set `PlayerController.bShowMouseCursor` true (`GameplayStatics.GetPlayerController` 0))
  (`GameplayStatics.SetGamePaused` true))

(fn `UserConstructionScript`
  (set `self.Current HP` (`self.Max HP`)))