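; Short-lived weapon attack actor that damages patrol enemies (BP_Enemy_Patrol) it touches.
; When ArcBox begins overlapping a patrol enemy, it applies fixed damage and destroys itself.
; It also destroys itself on a blocking hit, printing a "WALL" debug string, or once a Tick-accumulated timer passes a quarter second.
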(event `self.ReceiveBeginPlay`
  (set `self.Timer` 0.0))

(event `self.ReceiveTick`
  (params (DeltaSeconds :type "Float (single-precision)"))
  (bind _timer (`self.Timer`))
  (set `self.Timer` (+ DeltaSeconds _timer))
  (if (> _timer 0.25)
    (`self.K2_DestroyActor`)))

(event `self.ArcBox.OnComponentBeginOverlap`
  (params (OverlappedComponent :type "PrimitiveComponent Object Reference") (OtherActor :type "Actor Object Reference") (OtherComp :type "PrimitiveComponent Object Reference") (OtherBodyIndex :type Integer) (bFromSweep :type Boolean) (SweepResult :type "HitResult Structure (by ref)"))
  (bind _asbp_enemy_patrol (cast `/Game/Blueprints/Enemies/BP_Enemy_Patrol` OtherActor))
  (`/Game/Blueprints/BP_Damageable.Take Damage` _asbp_enemy_patrol 50.0)
  (`self.K2_DestroyActor`))

(event `self.ReceiveHit`
  (params (MyComp :type "PrimitiveComponent Object Reference") (Other :type "Actor Object Reference") (OtherComp :type "PrimitiveComponent Object Reference") (bSelfMoved :type Boolean) (HitLocation :type "Vector Structure") (HitNormal :type "Vector Structure") (NormalImpulse :type "Vector Structure") (Hit :type "HitResult Structure (by ref)"))
  (`KismetSystemLibrary.PrintString` "WALL")
  (`self.K2_DestroyActor`))

(fn `UserConstructionScript`)