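; BP_Shadow_Player is an interactable shadow that plays a dialogue, then unlocks an ability for the player.
; AbilityToUnlock selects the Hate, Rage or Fear dialogue array.
; Each Interact call advances Index and shows that line in a Dialogue widget, created when none is valid.
; After the last line it calls UnlockAbility on BP_Player, destroys itself and removes the widget; the Fear branch also opens the Outro level.
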(event `/Game/UI/BPI_Dialogue.Interact`
  (bind _abilitytounlock (`self.AbilityToUnlock`))
  (bind _asbp_player (cast `/Game/Blueprints/Character/BP_Player` (`GameplayStatics.GetPlayerCharacter` 0)))
  (if (`|EnumEquality` _abilitytounlock "NewEnumerator1")
    (if (<= (`self.Index`) (- (`KismetArrayLibrary.Array_Length` (`self.Hate Dialogue`)) 2))
      (`/Engine/EditorBlueprintResources/StandardMacros.IncrementInt` (`self.Index`)
        (:`  `
          (bind _ui (`self.UI`)
            (:`then`
              _)
            (:`else`
              (bind _returnvalue (`|CreateWidget` "/Game/UI/Dialogue.Dialogue_C" (`GameplayStatics.GetPlayerController` 0)))
              (bind _output_get (set `self.UI` _returnvalue))
              (`UserWidget.AddToViewport` _output_get 0)))
          (`TextBlock.SetText` (`/Game/UI/Dialogue.DialogueText` (`self.UI`)) (`KismetTextLibrary.Conv_StringToText` (`|GetArrayItem` (`self.Hate Dialogue`) (`self.Index`))))))
      (else
        (`/Game/Blueprints/Character/BP_Player.UnlockAbility` _asbp_player (`self.AbilityToUnlock`))
        (`self.K2_DestroyActor`)
        (`Widget.RemoveFromParent` _ui)))
    (elif (`|EnumEquality` _abilitytounlock "NewEnumerator2")
      (if (<= (`self.Index`) (- (`KismetArrayLibrary.Array_Length` (`self.Rage_Dialogue`)) 2))
        (`/Engine/EditorBlueprintResources/StandardMacros.IncrementInt` (`self.Index`)
          (:`  `
            (bind _ui_2 (`self.UI`)
              (:`then`
                _)
              (:`else`
                (bind _returnvalue_2 (`|CreateWidget` "/Game/UI/Dialogue.Dialogue_C" (`GameplayStatics.GetPlayerController` 0)))
                (bind _output_get_2 (set `self.UI` _returnvalue_2))
                (`UserWidget.AddToViewport` _output_get_2 0)))
            (`TextBlock.SetText` (`/Game/UI/Dialogue.DialogueText` (`self.UI`)) (`KismetTextLibrary.Conv_StringToText` (`|GetArrayItem` (`self.Rage_Dialogue`) (`self.Index`))))))
        (else
          (`/Game/Blueprints/Character/BP_Player.UnlockAbility` _asbp_player (`self.AbilityToUnlock`))
          (`self.K2_DestroyActor`)
          (`Widget.RemoveFromParent` _ui_2)))
      (elif (`|EnumEquality` _abilitytounlock "NewEnumerator3")
        (if (<= (`self.Index`) (- (`KismetArrayLibrary.Array_Length` (`self.Fear Dialogue`)) 2))
          (`/Engine/EditorBlueprintResources/StandardMacros.IncrementInt` (`self.Index`)
            (:`  `
              (bind _ui_3 (`self.UI`)
                (:`then`
                  _)
                (:`else`
                  (bind _returnvalue_3 (`|CreateWidget` "/Game/UI/Dialogue.Dialogue_C" (`GameplayStatics.GetPlayerController` 0)))
                  (bind _output_get_3 (set `self.UI` _returnvalue_3))
                  (`UserWidget.AddToViewport` _output_get_3 0)))
              (`TextBlock.SetText` (`/Game/UI/Dialogue.DialogueText` (`self.UI`)) (`KismetTextLibrary.Conv_StringToText` (`|GetArrayItem` (`self.Fear Dialogue`) (`self.Index`))))))
          (else
            (`/Game/Blueprints/Character/BP_Player.UnlockAbility` _asbp_player (`self.AbilityToUnlock`))
            (`self.K2_DestroyActor`)
            (`Widget.RemoveFromParent` _ui_3)
            (`GameplayStatics.OpenLevelBySoftObjectPtr` "/Game/Levels/Outro.Outro")))))))

(fn `UserConstructionScript`)