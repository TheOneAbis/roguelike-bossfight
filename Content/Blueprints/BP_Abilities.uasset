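; Ability Blueprint that defines three callable player abilities as events: Basic, Hate and Rage.
; Basic finds BP_Player by class and briefly enables overlap events on its AttackBox as a timed hit window, with the swing animation still to be added.
; Hate spawns an Arc actor at the ArcPoint world transform.
; Rage is a stub that only prints its name.
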(event `Basic`
  (bind _returnvalue (`GameplayStatics.GetActorOfClass` "/Game/Blueprints/Character/BP_Player.BP_Player_C"))
  (bind _attackbox (`/Game/Blueprints/Character/BP_Player.AttackBox` _returnvalue))
  (set `PrimitiveComponent.bGenerateOverlapEvents` true _attackbox)
  (`KismetSystemLibrary.Delay` 0.2) ; Need basic swing animation
  (set `PrimitiveComponent.bGenerateOverlapEvents` false _attackbox))

(event `Hate`
  (`|SpawnActorFromClass` "/Game/Blueprints/Weapon/Arc.Arc_C" (`SceneComponent.K2_GetComponentToWorld` (`self.ArcPoint`)) "Undefined" "MultiplyWithRoot" null null))

(event `Rage`
  (`KismetSystemLibrary.PrintString` "Rage"))

(fn `UserConstructionScript`
  (`parent.UserConstructionScript`))