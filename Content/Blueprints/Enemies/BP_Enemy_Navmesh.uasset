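; BP_Enemy_Navmesh is an enemy Blueprint that chases the player and dies when its health runs out.
; Tick issues AIMoveTo toward the Player reference every frame, which this file never assigns.
; Construction sets CurrentHP to MaxHP, and TakeDamage subtracts damage and destroys the actor at zero or below.
; The AttackSphere overlap checks for the player, but the attack itself is an empty stub.
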(event `self.ReceiveBeginPlay`)

(event `self.ReceiveTick`
  (params (DeltaSeconds :type "Float (single-precision)"))
  ;[1 0.8747 0.3581] Chases the player down. Attacking the player once in range is handled in the AttackSphere begin overlap event
  (`|AIMoveTo` self (0.0 0.0 0.0) (`self.player`) 20.0))

(event `Take Damage`
  (params (damage :type "Float (double-precision)"))
  (bind _current_hp (`self.current HP`))
  ;[1 0.4531 0.4531] Taking damage. If hp <= 0, this enemy is dead and destroyed.
  (set `self.current HP` (- _current_hp damage))
  (if (<= _current_hp 0.0)
    (`self.K2_DestroyActor`)))

(event `self.AttackSphere.OnComponentBeginOverlap`
  (params (OverlappedComponent :type "PrimitiveComponent Object Reference") (OtherActor :type "Actor Object Reference") (OtherComp :type "PrimitiveComponent Object Reference") (OtherBodyIndex :type Integer) (bFromSweep :type Boolean) (SweepResult :type "HitResult Structure (by ref)"))
  (if (== OtherActor (`self.player`))
    _))

(fn `UserConstructionScript`
  (set `self.current HP` (`self.Max HP`)))