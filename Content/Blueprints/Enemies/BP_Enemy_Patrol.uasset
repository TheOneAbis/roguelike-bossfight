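; Enemy that patrols a looping point list, chases the player on sight, and respawns at its current patrol point when killed.
; Tick detects the player by range, view-cone dot product and line trace, then moves toward the last seen position, resuming patrol on arrival.
; AttackCollider overlap runs a delayed damage loop until the player leaves or dies, opening the death menu on death.
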(event `OnKilled`
  (`self.K2_SetActorLocation` (`self.K2_GetActorLocation` (`|GetArrayItem` (`self.PatrolPoints`) (`self.currentPt`))) false true)
  (set `self.Current HP` (`self.Max HP`))
  (set `self.Dead` false)
  (`self.Set Patrolling`)
  (`KismetSystemLibrary.DelayUntilNextTick`)
  (set `self.attacking` false)
  (`MovementComponent.StopMovementImmediately` (`self.CharacterMovement`)))

(event `self.ReceiveBeginPlay`
  (add `self.OnKilledDispatch` (delegate `OnKilled`))
  (set `CharacterMovementComponent.MaxWalkSpeed` (`self.patrolling speed`) (`self.CharacterMovement`))
  (`self.Begin Patrolling`))

(event `Begin Patrolling`
  (bind _output (`|GetArrayItem` (`self.PatrolPoints`) (`self.currentPt`)))
  (`/Engine/EditorBlueprintResources/StandardMacros.IsValid` _output :!label _label ; If the patrol point at this index is invalid, we may have hit the end of the list, so reset back to the front.
    (:`Is Valid`
      (if (== (`self.patrolState`) 0)
        (`|AIMoveTo` self (0.0 0.0 0.0) _output 20.0
          (:`OnSuccess`
            (`/Engine/EditorBlueprintResources/StandardMacros.IncrementInt` (`self.currentPt`)
              (:`  `
                (goto _label)))))))
    (:`Is Not Valid`
      (set `self.currentPt` 0)
      (`/Engine/EditorBlueprintResources/StandardMacros.IsValid` _output ; If the first item is invalid, the patrol list is empty, so stop here.
        (:`Is Valid`
          (goto _label))
        (:`Is Not Valid`
          (`KismetSystemLibrary.PrintString` "WARNING: The patrol points list on this enemy is empty. This enemy will not move."))))))

(event `self.ReceiveTick`
  (params (DeltaSeconds :type "Float (single-precision)"))
  (bind _returnvalue (`GameplayStatics.GetPlayerPawn` 0))
  (bind _returnvalue_2 (`GameplayStatics.GetPlayerPawn` 0))
  (bind _returnvalue_3 (`GameplayStatics.GetPlayerPawn` 0))
  (bind _returnvalue_4 (- (`self.K2_GetActorLocation` _returnvalue) (`self.K2_GetActorLocation`)))
  (`/Engine/EditorBlueprintResources/StandardMacros.IsValid` _returnvalue
    (:`Is Valid`
      (switch `int` (`self.patrolState`)
        (:`0`
          (if (<= (`KismetMathLibrary.VSizeSquared` _returnvalue_4) (`KismetMathLibrary.Square` (`self.detectionRange`)))
            (if (>= (`KismetMathLibrary.Dot_VectorVector` (`KismetMathLibrary.Normal` _returnvalue_4) (`self.GetActorForwardVector`)) (`KismetMathLibrary.DegCos` (`self.detectionAngleDeg`)))
              (bind _outhit (`KismetSystemLibrary.LineTraceSingleForObjects` (`self.K2_GetActorLocation`) (`self.K2_GetActorLocation` _returnvalue_3) (`self.objecttypes`)))
              (if (== (`.HitActor` (`GameplayStatics.BreakHitResult` _outhit)) _returnvalue_3)
                (`self.Set Chasing`)))))
        (:`1`
          (bind _outhit_2 (`KismetSystemLibrary.LineTraceSingleForObjects` :`Start` (`self.K2_GetActorLocation`) :`End` (`self.K2_GetActorLocation` _returnvalue_2) :`ObjectTypes` (`self.objecttypes`) :`DrawDebugType` "ForOneFrame"))
          (if (== (`.HitActor` (`GameplayStatics.BreakHitResult` _outhit_2)) _returnvalue_2)
            (`|AIMoveTo` self (`.Location` (`GameplayStatics.BreakHitResult` _outhit_2)) null 20.0
              (:`OnSuccess`
                (`self.Set Patrolling`)))))))
    (:`Is Not Valid`
      (`self.SetActorTickEnabled` false))))

(event `self.AttackCollider.OnComponentBeginOverlap`
  (params (OverlappedComponent :type "PrimitiveComponent Object Reference") (OtherActor :type "Actor Object Reference") (OtherComp :type "PrimitiveComponent Object Reference") (OtherBodyIndex :type Integer) (bFromSweep :type Boolean) (SweepResult :type "HitResult Structure (by ref)"))
  (bind _returnvalue (`GameplayStatics.GetPlayerPawn` 0))
  (if (== OtherActor _returnvalue)
    (set `self.attacking` true)
    (`KismetSystemLibrary.RetriggerableDelay` 1.0 :!label _label_2)
    (if (`self.attacking`)
      (bind _asbp_damageable (cast `/Game/Blueprints/BP_Damageable` _returnvalue))
      (`self.Take Damage` _asbp_damageable 28.0)
      (if (`/Game/Blueprints/BP_Damageable.Dead` _asbp_damageable)
        (`self.DeathMenu`)
        (else
          (goto _label_2))))))

(event `self.AttackCollider.OnComponentEndOverlap`
  (params (OverlappedComponent :type "PrimitiveComponent Object Reference") (OtherActor :type "Actor Object Reference") (OtherComp :type "PrimitiveComponent Object Reference") (OtherBodyIndex :type Integer))
  (if (== (`GameplayStatics.GetPlayerPawn` 0) OtherActor)
    (set `self.attacking` false)))

(event `Set Chasing`
  (set `self.patrolState` 1)
  (set `CharacterMovementComponent.MaxWalkSpeed` (`self.chasing speed`) (`self.CharacterMovement`)))

(event `Set Patrolling`
  (set `self.patrolState` 0)
  (set `CharacterMovementComponent.MaxWalkSpeed` (`self.patrolling speed`) (`self.CharacterMovement`))
  (`self.Begin Patrolling`))

(fn `UserConstructionScript`
  (`parent.UserConstructionScript`))