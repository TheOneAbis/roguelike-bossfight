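; Melee enemy Blueprint that chases the player and deals repeated damage while in attack range.
; Tick reissues AIMoveTo toward the player pawn every frame.
; AttackCollider overlaps toggle an Attacking flag, and begin overlap starts a Delay loop that damages the player through a BP_Damageable cast after each wait.
; The loop stops once Attacking clears or the player dies, with death calling DeathMenu.
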(event `self.ReceiveTick`
  (params (DeltaSeconds :type "Float (single-precision)"))
  (bind _returnvalue (`GameplayStatics.GetPlayerPawn` 0))
  ;[1 0.8747 0.3581] Chases the player down. Attacking the player once in range is handled in the AttackSphere begin overlap event
  (`/Engine/EditorBlueprintResources/StandardMacros.IsValid` _returnvalue
    (:`Is Valid`
      (`|AIMoveTo` self (0.0 0.0 0.0) _returnvalue 20.0))))

(event `self.AttackCollider.OnComponentBeginOverlap`
  (params (OverlappedComponent :type "PrimitiveComponent Object Reference") (OtherActor :type "Actor Object Reference") (OtherComp :type "PrimitiveComponent Object Reference") (OtherBodyIndex :type Integer) (bFromSweep :type Boolean) (SweepResult :type "HitResult Structure (by ref)"))
  (bind _returnvalue (`GameplayStatics.GetPlayerPawn` 0))
  (if (== OtherActor _returnvalue)
    (set `self.attacking` true)
    (`KismetSystemLibrary.Delay` 1.0 :!label _label) ; Attacking every 2 seconds
    (if (`self.attacking`)
      (bind _asbp_damageable (cast `/Game/Blueprints/BP_Damageable` _returnvalue))
      (`self.Take Damage` _asbp_damageable 50.0)
      (if (`/Game/Blueprints/BP_Damageable.Dead` _asbp_damageable)
        (`self.DeathMenu`)
        (else
          (goto _label))))))

(event `self.AttackCollider.OnComponentEndOverlap`
  (params (OverlappedComponent :type "PrimitiveComponent Object Reference") (OtherActor :type "Actor Object Reference") (OtherComp :type "PrimitiveComponent Object Reference") (OtherBodyIndex :type Integer))
  (if (== (`GameplayStatics.GetPlayerPawn` 0) OtherActor)
    (set `self.attacking` false)))

(fn `UserConstructionScript`
  (`parent.UserConstructionScript`))